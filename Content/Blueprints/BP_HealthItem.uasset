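; BP_HealthItem is an interactable health pickup that heals the player character when used.
; On interaction it casts the character to BP_YinCharacter, calls Heal with a fixed amount, then destroys itself.
; A sphere trigger shows a widget while an actor tagged Player overlaps it and hides it when that actor leaves.
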(event OnComponentBeginOverlap(Sphere)
  (params (OverlappedComponent :type Primitive%20Component%20Object%20Reference) (OtherActor :type Actor%20Object%20Reference) (OtherComp :type Primitive%20Component%20Object%20Reference) (OtherBodyIndex :type Integer) (bFromSweep :type Boolean) (SweepResult :type Hit%20Result%20Structure%20%28by%20ref%29))
  ;[0 0.3333 1] Widget overlap manager
  (if (Actor|ActorHasTag OtherActor "Player")
    (Rendering|SetVisibility (Variables|Default|GetWidget) true false)))

(event OnComponentEndOverlap(Sphere)
  (params (OverlappedComponent :type Primitive%20Component%20Object%20Reference) (OtherActor :type Actor%20Object%20Reference) (OtherComp :type Primitive%20Component%20Object%20Reference) (OtherBodyIndex :type Integer))
  ;[0 0.3333 1] Widget overlap manager
  (if (Actor|ActorHasTag OtherActor "Player")
    (Rendering|SetVisibility (Variables|Default|GetWidget) false false)))

(event EventBeginPlay)

(event EventTick
  (params (DeltaSeconds :type Float%20%28single-precision%29)))

(event EventOnInteraction
  (params (character :type D3D%20Character%20Base%20Object%20Reference))
  ;[1 0.6084 0] HealPlayer
  (bind _asbp_yin_character (Utilities|Casting|CastToBP_YinCharacter character))
  (Default|Heal _asbp_yin_character 5e+01)
  (Actor|DestroyActor))

(fn ConstructionScript)