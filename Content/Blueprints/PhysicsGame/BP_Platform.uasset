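; BP_Platform is a moving platform that oscillates up and down around the location where it begins play.
; BeginPlay stores that initial location, and Tick accumulates elapsed time to drive a sine wave on the Z axis.
; A Direction variable multiplies the fixed-amplitude offset, while X and Y stay at their starting values.
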(event EventBeginPlay
  (Variables|Default|SetInitialPosition (Transformation|GetActorLocation)))

(event Collision|EventActorBeginOverlap
  (params (OtherActor :type Actor%20Object%20Reference)))

(event EventTick
  (params (DeltaSeconds :type Float%20%28single-precision%29))
  (bind _initialposition (Variables|Default|GetInitialPosition))
  (bind _output_get (Variables|Default|SetElpasedTime (+ DeltaSeconds (Variables|Default|GetElpasedTime))))
  (Transformation|SetActorLocation (Math|Vector|MakeVector (.x _initialposition) (.y _initialposition) (+ (.z _initialposition) (* (* (Math|Trig|Sin(Radians) _output_get) 1e+02) (Variables|Default|GetDirection)))) false false))

(fn ConstructionScript)