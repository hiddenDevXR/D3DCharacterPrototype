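; BP_Ball is a physics ball that reacts to tagged actors it hits in the physics game.
; On BeginPlay it binds to its own hit event and checks the other actor's tags in priority order.
; SpeedPad pushes the mesh along world +Y and JumpBoost launches it upward, both as mass-dependent impulses.
; Destructible fires the RadialForce component's impulse.
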(event Custom|OnActorHit_Event
  (params (SelfActor :type Actor%20Object%20Reference) (OtherActor :type Actor%20Object%20Reference) (NormalImpulse :type Vector) (Hit :type Hit%20Result%20Structure%20%28by%20ref%29))
  (if (Actor|ActorHasTag OtherActor "SpeedPad")
    (Physics|AddImpulse (Variables|Debug|GetStaticMeshComponent) "0.000000,10000.000000,0.000000" "None" false)
    (elif (Actor|ActorHasTag OtherActor "JumpBoost")
      (Physics|AddImpulse (Variables|Debug|GetStaticMeshComponent) "0.000000,0.000000,80000.000000" "None" false)
      (elif (Actor|ActorHasTag OtherActor "Destructible")
        (Class|RadialForceComponent|FireImpulse (Variables|Default|GetRadialForce))))))

(event EventBeginPlay
  (Collision|AssignOnActorHit (delegate Custom|OnActorHit_Event)))

(event Collision|EventActorBeginOverlap
  (params (OtherActor :type Actor%20Object%20Reference)))

(event EventTick
  (params (DeltaSeconds :type Float%20%28single-precision%29)))

(fn ConstructionScript)