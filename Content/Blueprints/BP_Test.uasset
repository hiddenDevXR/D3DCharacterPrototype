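; BP_Test is an interactable door that swings open and closed and shows a widget when the player is near.
; OnInteraction plays or reverses the Opening timeline based on IsClosed, lerping the Pivot's yaw between 0 and 90 degrees and toggling IsClosed on finish.
; A Sphere component's begin and end overlaps show and hide the Widget for actors tagged Player.
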(event OnComponentBeginOverlap(Sphere)
  (params (OverlappedComponent :type Primitive%20Component%20Object%20Reference) (OtherActor :type Actor%20Object%20Reference) (OtherComp :type Primitive%20Component%20Object%20Reference) (OtherBodyIndex :type Integer) (bFromSweep :type Boolean) (SweepResult :type Hit%20Result%20Structure%20%28by%20ref%29))
  ;[0 0.3333 1] Widget overlap manager
  (if (Actor|ActorHasTag OtherActor "Player")
    (Rendering|SetVisibility (Variables|Default|GetWidget) true false)))

(event OnComponentEndOverlap(Sphere)
  (params (OverlappedComponent :type Primitive%20Component%20Object%20Reference) (OtherActor :type Actor%20Object%20Reference) (OtherComp :type Primitive%20Component%20Object%20Reference) (OtherBodyIndex :type Integer))
  ;[0 0.3333 1] Widget overlap manager
  (if (Actor|ActorHasTag OtherActor "Player")
    (Rendering|SetVisibility (Variables|Default|GetWidget) false false)))

(event EventBeginPlay)

(event EventOnInteraction
  (params (Player :type BP%20Third%20Person%20Character%20Object%20Reference))
  ;[1 0.6084 0] Door animation
  (if (Variables|Default|GetIsClosed)
    (bind _doorangle (Timeline|Opening PlayFromStart)
      (:Update
        (Transformation|SetRelativeRotation (Variables|Default|GetPivot) (Math|Rotator|MakeRotator 0.0 0.0 (Math|Float|Lerp 0.0 9e+01 _doorangle)) false false))
      (:Finished
        (Variables|Default|SetIsClosed (not (Variables|Default|GetIsClosed)))))
    (else
      (Timeline|Opening Reverse))))

(event EventTick
  (params (DeltaSeconds :type Float%20%28single-precision%29)))

(fn ConstructionScript)