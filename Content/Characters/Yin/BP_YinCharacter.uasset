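; BP_YinCharacter is the Blueprint for the Yin character, handling its health HUD, ability animation and debug emotes.
; BeginPlay creates W_HUDTest and binds damage and death events, refreshing health as a fraction of 100 and printing the death cause.
; Heal raises the Health attribute's base value but sends the HUD an unnormalized sum, unlike the damage path.
; IA_Fire plays the ability montage, and two debug keys play emote sections.
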(event Custom|On%20Die
  (params (Cause :type ED3DDeathCause%20Enum :default "None"))
  (Development|PrintString (Utilities|String|EnumtoString Cause)))

(event Custom|OnTakeAnyDamage_Event_0
  (params (DamagedActor :type Actor%20Object%20Reference) (Damage :type Float%20%28single-precision%29) (DamageType :type Damage%20Type%20Object%20Reference) (InstigatedBy :type Controller%20Object%20Reference) (DamageCauser :type Actor%20Object%20Reference))
  (bind _healthpercentage (CallFunction|GetHealthPercentage))
  (Default|UpdateHealth (Variables|Default|GetHUD) _healthpercentage))

(event Input|EnhancedActionEvents|EnhancedInputActionIA_Fire
  (params (ActionValue :type Boolean) (ElapsedSeconds :type Float%20%28double-precision%29) (TriggeredSeconds :type Float%20%28double-precision%29) (InputAction :type Input%20Action%20Object%20Reference :default "/Game/ThirdPerson/Input/Actions/IA_Fire.IA_Fire"))
  (Animation|PlayAnimMontage "/Game/Characters/Yin/Animations/AM_Yin_Ability.AM_Yin_Ability" 1.0 ""))

(event EventBeginPlay
  (|CallParentFunction)
  (EventDispatchers|BindEventtoOnDie (delegate Custom|On%20Die))
  (bind _returnvalue (UserInterface|CreateWidget "/Game/Blueprints/UI/W_HUDTest.W_HUDTest_C"))
  (bind _output_get (Variables|Default|SetHUD _returnvalue))
  (UserInterface|Viewport|AddtoViewport _output_get 0)
  (EventDispatchers|AssignOnTakeAnyDamage (delegate Custom|OnTakeAnyDamage_Event_0)))

(event Collision|EventActorBeginOverlap
  (params (OtherActor :type Actor%20Object%20Reference))
  (|CallParentFunction OtherActor) ; This node is disabled and will not be called.\nDrag off pins to build functionality.
)

(event EventTick
  (params (DeltaSeconds :type Float%20%28single-precision%29))
  (|CallParentFunction DeltaSeconds))

(event Input|KeyboardEvents|DebugKey3
  (params (Key :type Key%20Structure :default "None") (ActionValue :type Input%20Action%20Value%20Structure))
  (:Pressed
    (Animation|PlayAnimMontage "/Game/Characters/Yin/Animations/AM_Yin_Emote.AM_Yin_Emote" 1.0 "Indie")))

(event Input|KeyboardEvents|DebugKey4
  (params (Key :type Key%20Structure :default "None") (ActionValue :type Input%20Action%20Value%20Structure))
  (:Pressed
    (Animation|PlayAnimMontage "/Game/Characters/Yin/Animations/AM_Yin_Emote.AM_Yin_Emote" 1.0 "Squash")))

(fn ConstructionScript
  (|CallParentFunction))

(fn GetHealthPercentage
  (return (/ (.BaseValue (Utilities|Struct|BreakD3DGameplayAttribute (Variables|/Script/PrototypeBP.D3DCharacterAttributeComponent|GetHealth (Class|D3DCharacterBase|GetAttributes)))) 1e+02)))

(fn Heal
  (params (HealAmount :type Float%20%28double-precision%29))
  (bind _returnvalue (Class|D3DCharacterBase|GetAttributes))
  (bind _health (Variables|/Script/PrototypeBP.D3DCharacterAttributeComponent|GetHealth _returnvalue))
  (bind _basevalue (Utilities|Struct|BreakD3DGameplayAttribute _health))
  (bind _returnvalue_2 (+ _basevalue HealAmount))
  (Class|D3DGameplayAttributesLibrary|SetBaseValue _health _returnvalue_2)
  (Default|UpdateHealth (Variables|Default|GetHUD) _returnvalue_2))