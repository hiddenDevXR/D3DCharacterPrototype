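; BP_PhaseCharacter is the Phase character Blueprint, adding death logging and debug animation keys to its parent class.
; On BeginPlay it runs the parent logic and binds OnDie, which prints the death cause enum on screen.
; Debug keys play named sections of the emote montage or the ability montage directly.
; Overlap and Tick are disabled stubs, and construction only calls the parent.
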(event Custom|On%20Die
  (params (Cause :type ED3DDeathCause%20Enum :default "None"))
  (Development|PrintString (Utilities|String|EnumtoString Cause)))

(event EventBeginPlay
  (|CallParentFunction)
  (EventDispatchers|BindEventtoOnDie (delegate Custom|On%20Die)))

(event Collision|EventActorBeginOverlap
  (params (OtherActor :type Actor%20Object%20Reference))
  (|CallParentFunction OtherActor) ; This node is disabled and will not be called.\nDrag off pins to build functionality.
)

(event EventTick
  (params (DeltaSeconds :type Float%20%28single-precision%29))
  (|CallParentFunction DeltaSeconds) ; This node is disabled and will not be called.\nDrag off pins to build functionality.
)

(event Input|KeyboardEvents|DebugKey3
  (params (Key :type Key%20Structure :default "None") (ActionValue :type Input%20Action%20Value%20Structure))
  (:Pressed
    (Animation|PlayAnimMontage "/Game/Characters/Phase/Animations/AM_Emote.AM_Emote" 1.0 "STFU")))

(event Input|KeyboardEvents|DebugKey4
  (params (Key :type Key%20Structure :default "None") (ActionValue :type Input%20Action%20Value%20Structure))
  (:Pressed
    (Animation|PlayAnimMontage "/Game/Characters/Phase/Animations/AM_Emote.AM_Emote" 1.0 "Break")))

(event Input|KeyboardEvents|DebugKeyH
  (params (Key :type Key%20Structure :default "None") (ActionValue :type Input%20Action%20Value%20Structure))
  (:Pressed
    (Animation|PlayAnimMontage "/Game/Characters/Phase/Animations/AM_Ability.AM_Ability" 1.0 "")))

(fn ConstructionScript
  (|CallParentFunction))